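; Player character Blueprint whose construction script hides both upper arm bones and the neck bone on the mesh, removing arms and head from view.
; The event graph has no active logic, as Tick is empty.
; Disconnected nodes remain from an unfinished surface check that traces downward from the actor, prints the physical surface type and switches on it.
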(event `self.ReceiveTick`
  (params (DeltaSeconds :type "Float (single-precision)")))

(fn `UserConstructionScript`
  (bind _mesh (`self.Mesh`))
  (`SkinnedMeshComponent.HideBoneByName` _mesh "upperarm_r" "PBO_None")
  (`SkinnedMeshComponent.HideBoneByName` _mesh "upperarm_l" "PBO_None")
  (`SkinnedMeshComponent.HideBoneByName` _mesh "neck_01" "PBO_None"))