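; Demo actor that previews a crafting printer effect, with a Niagara beam and a dissolve on a test mesh.
; BeginPlay calls Craft, which plays a timeline driving the mesh's DissolveAmount material parameter.
; The same timeline's ZigZagMotion, scaled by Amplitude and offset from the mesh's location, moves the beam end to sweep like a print head.
; The construction script resets the dissolve and aims the beam at the mesh.
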(event `self.ReceiveBeginPlay`
  (`self.Craft`))

(event `Craft`
  (bind _testcraftingmesh (`self.TestCraftingMesh`))
  (bind (_direction _dissolveprogress _zigzagmotion) (`Timeline|Timeline`)
    (:`Update`
      (`MeshComponent.SetScalarParameterValueOnMaterials` _testcraftingmesh "DissolveAmount" _dissolveprogress)
      (`NiagaraComponent.SetNiagaraVariableVec3` (`self.CraftingBeam`) "User.BeamEndVec" (+ (* _zigzagmotion (`self.Amplitude`)) (`SceneComponent.K2_GetComponentLocation` _testcraftingmesh))))))

(fn `UserConstructionScript`
  (bind _testcraftingmesh (`self.TestCraftingMesh`))
  (`MeshComponent.SetScalarParameterValueOnMaterials` _testcraftingmesh "DissolveAmount" 0.0)
  (`NiagaraComponent.SetNiagaraVariableVec3` (`self.CraftingBeam`) "User.BeamEndVec" (`SceneComponent.K2_GetComponentLocation` _testcraftingmesh)))